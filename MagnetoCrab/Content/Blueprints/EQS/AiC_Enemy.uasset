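; AI controller for enemies that runs the BT_Enemy behavior tree on possess and tracks the player through AI perception.
; Sensing an actor tagged Player sets the HasLineOfSight and TargetActor blackboard keys and cancels any pending lost-sight timer.
; Losing the player clears HasLineOfSight at once, while TargetActor is cleared only after a delay of several seconds, so the enemy briefly remembers its target.
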(event OnTargetPerceptionUpdated(AIPerception)
  (params (Actor :type Actor%20Object%20Reference) (Stimulus :type AI%20Stimulus%20Structure))
  (Variables|Default|SetPerceivedActor Actor)
  (if (Actor|ActorHasTag Actor "Player")
    (if (Utilities|Struct|BreakAIStimulus Stimulus)
      (Utilities|Time|ClearandInvalidateTimerbyHandle (Variables|Default|GetLostSightTimer))
      (CallFunction|UpdateSightKey true)
      (CallFunction|UpdateTargetKey (Variables|Default|GetPerceivedActor))
      (else
        (bind _returnvalue (Utilities|Time|SetTimerbyEvent (delegate Custom|LostSight) 8.0))
        (Variables|Default|SetLostSightTimer _returnvalue)
        (CallFunction|UpdateSightKey false)))))

(event Custom|LostSight
  (CallFunction|UpdateTargetKey))

(event EventBeginPlay)

(event EventTick
  (params (DeltaSeconds :type Float%20%28single-precision%29)))

(event EventPossess
  (params (PossessedPawn :type Pawn%20Object%20Reference))
  (AI|RunBehaviorTree "/Game/Blueprints/EQS/BT_Enemy.BT_Enemy"))

(fn ConstructionScript)

(fn UpdateSightKey
  (params (HasLineOfSight :type Boolean))
  (AI|Components|Blackboard|SetValueasBool (Variables|Default|GetBlackboard) (Utilities|Name|MakeLiteralName "HasLineOfSight") HasLineOfSight))

(fn UpdateTargetKey
  (params (TargetActor :type Actor%20Object%20Reference))
  (AI|Components|Blackboard|SetValueasObject (Variables|Default|GetBlackboard) (Utilities|Name|MakeLiteralName "TargetActor") TargetActor))