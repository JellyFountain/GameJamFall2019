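; BP_AiCharacter is an AI character that roams the level and chases the player on sight.
; It repeatedly moves to random navigable points near its current location, pausing briefly between moves.
; When PawnSensing sees a WyattsFirstPersonCharacter, it moves to that player, then disables sensing and waits before resuming roaming, which re-enables sensing.
; Move requests only handle success, so a failed move does not restart the loop.
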(event OnSeePawn(PawnSensing)
  (params (Pawn :type Pawn%20Object%20Reference))
  ;[1 1 1] Chase player on sight
  (bind _aswyatts_first_person_character (Utilities|Casting|CastToWyattsFirstPersonCharacter Pawn))
  (CallFunction|ChasePlayer _aswyatts_first_person_character))

(event Custom|MoveToRandomLocation
  ;[1 1 1] Roam
  (Class|PawnSensingComponent|SetSensingUpdatesEnabled (Variables|Default|GetPawnSensing) true)
  (AI|AIMoveTo self (.RandomLocation (Class|NavigationSystemV1|GetRandomPointinNavigableRadius (Transformation|GetActorLocation) 5e+02 0 0)) 0 5.0 false
    (:OnSuccess
      (Utilities|FlowControl|Delay 0.5)
      (CallFunction|MovetoRandomLocation))))

(event Custom|Chase%20Player
  (params (Player%20to%20Chase :type Pawn%20Object%20Reference))
  ;[1 1 1] Move to player then stop for x time
  (AI|AIMoveTo self "0, 0, 0" Player%20to%20Chase 1e+01 false
    (:OnSuccess
      (Class|PawnSensingComponent|SetSensingUpdatesEnabled (Variables|Default|GetPawnSensing) false)
      (Utilities|FlowControl|Delay 3.0)
      (CallFunction|MovetoRandomLocation))))

(event EventBeginPlay
  ;[1 1 1] Start
  (CallFunction|MovetoRandomLocation))

(fn ConstructionScript)