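; Magnetic object actor that can be pushed away from or pulled toward a given actor.
; MagneticPush and MagneticPull set state flags and disable gravity, and StopMagnetic clears the flags.
; Tick moves the Sphere by a fixed per-frame step without sweep, with push taking priority, and restores gravity when idle.
; A pulled object attaches to the hold location once its largest axis distance drops below the minimum, detaching while farther away.
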(event Custom|MagPush
  ;[1 1 1] Push
  (Physics|SetEnableGravity (Variables|Default|GetSphere) false))

(event Custom|MagPull
  ;[1 1 1] Pull
  (Physics|SetEnableGravity (Variables|Default|GetSphere) false))

(event EventBeginPlay)

(event Collision|EventActorBeginOverlap
  (params (OtherActor :type Actor%20Object%20Reference)))

(event EventTick
  (params (DeltaSeconds :type Float%20%28single-precision%29))
  (bind _sphere (Variables|Default|GetSphere))
  (bind _sphere_2 (Variables|Default|GetSphere))
  ;[1 1 1] If the object is being pushed
  (if (Variables|Default|GetBeingPushed)
    ;[1 1 1] Push
    (Transformation|SetWorldLocation _sphere (- (Transformation|GetWorldLocation _sphere) (* (Math|Vector|Normalize (- (Transformation|GetWorldLocation (Variables|Default|GetActorToMoveAwayFrom)) (Transformation|GetWorldLocation _sphere))) (Variables|Default|GetMoveSpeed))) false false)
    (else
      ;[1 1 1] If the object is being pulled
      (if (Variables|Default|GetBeingPulled)
        ;[1 1 1] Pull
        (if (>= (Math|Vector|GetMaxElement (Math|Vector|VectorGetAbs (- (Transformation|GetWorldLocation (Variables|Default|GetSphere)) (Transformation|GetWorldLocation (Variables|Default|GetActorToMoveAwayFrom))))) (Variables|Default|GetMinimum%20Distance))
          (Transformation|DetachFromActor "KeepWorld" "KeepWorld" "KeepWorld")
          (Transformation|SetWorldLocation _sphere_2 (+ (Transformation|GetWorldLocation _sphere_2) (* (Math|Vector|Normalize (- (Transformation|GetWorldLocation (Variables|Default|GetActorToMoveAwayFrom)) (Transformation|GetWorldLocation _sphere_2))) (Variables|Default|GetMoveSpeed))) false false)
          (else
            (Physics|SetEnableGravity (Variables|Default|GetSphere) false)
            (Transformation|AttachComponentToComponent (Variables|Default|GetHoldLocationActor) "None" "KeepRelative" "KeepWorld" "KeepWorld" true)))
        (else
          ;[1 1 1] If neither, then give it gravity
          (Physics|SetEnableGravity (Variables|Default|GetSphere) true))))))

(fn ConstructionScript)

(fn MagneticPush
  (params (ActorToMoveAwayFrom :type Static%20Mesh%20Component%20Object%20Reference))
  (Variables|Default|SetBeingPushed true)
  (Variables|Default|SetActorToMoveAwayFrom ActorToMoveAwayFrom)
  (CallFunction|MagPush))

(fn MagneticPull
  (params (ActorToMoveAwayFrom :type Static%20Mesh%20Component%20Object%20Reference) (HoldLocationActor :type Static%20Mesh%20Component%20Object%20Reference))
  (Variables|Default|SetBeingPulled true)
  (Variables|Default|SetActorToMoveAwayFrom ActorToMoveAwayFrom)
  (Variables|Default|SetHoldLocationActor HoldLocationActor)
  (CallFunction|MagPull))

(fn StopMagnetic
  (Variables|Default|SetBeingPushed false)
  (Variables|Default|SetBeingPulled false)
  (Development|PrintString "StopMagnetic"))